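; BP_Rocket is a short-lived projectile that damages actors tagged as targets.
; It expires a few seconds after spawning.
; On overlapping a target, it applies damage credited to the first player controller, plays explosion sound and particles at its location, then calls GameCheck on BP_Gamemode and destroys itself.
; If the game mode cast fails, the rocket is not destroyed on impact.
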(event EventBeginPlay
  (Actor|SetLifeSpan 3.0))

(event Collision|EventActorBeginOverlap
  (params (OtherActor :type Actor%20Object%20Reference))
  (bind _returnvalue (Transformation|GetActorLocation))
  (if (Actor|ActorHasTag OtherActor "Target")
    (Game|Damage|ApplyDamage OtherActor 1e+02 (Game|GetPlayerController 0) self)
    (Audio|SpawnSoundatLocation "/Game/StarterContent/Audio/Explosion_Cue.Explosion_Cue" _returnvalue "0, 0, 0" 1.0 1.0 0.0 0 0)
    (Effects|SpawnEmitteratLocation "/Game/StarterContent/Particles/P_Explosion.P_Explosion" _returnvalue)
    (bind _asbp_gamemode (Utilities|Casting|CastToBP_Gamemode (Game|GetGameMode)))
    (Default|GameCheck _asbp_gamemode)
    (Actor|DestroyActor)))

(fn ConstructionScript)